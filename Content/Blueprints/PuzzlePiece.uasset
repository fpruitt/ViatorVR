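; Puzzle piece actor in an ordered chain puzzle, activated when it receives focus.
; On focus it turns green and completes if it has no previous piece or that piece is completed; the last piece then fires puzzle completion.
; Focusing out of order calls Reset, which turns the piece red and recurses back through the previous pieces to clear them.
; Blur and interact events are empty.
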(event EventOnFocus
  (bind _previouspiece (Variables|Default|GetPreviousPiece))
  (Utilities|IsValid _previouspiece
    (:Is%20Valid
      (if (Variables|PuzzlePiece_C|GetIsCompleted _previouspiece)
        (Variables|Default|SetIsCompleted true :!label _label)
        (Rendering|Material|SetVectorParameterValueonMaterials (Variables|Default|GetCube) "Color" "0.000000,1.000000, 0")
        (if (Variables|Default|GetIsLastPiece)
          (Default|CallPuzzleComplete)
          (Development|PrintString "Hello"))
        (else
          (CallFunction|Reset))))
    (:Is%20Not%20Valid
      (goto _label))))

(event EventOnBlur)

(event EventOnInteract)

(fn ConstructionScript
  (Rendering|Material|SetVectorParameterValueonMaterials (Variables|Default|GetCube) "Color" "1.000000,0.000000, 0"))

(fn Reset
  (bind _previouspiece (Variables|Default|GetPreviousPiece))
  (Rendering|Material|SetVectorParameterValueonMaterials (Variables|Default|GetCube) "Color" "1.000000,0.000000, 0")
  (Variables|Default|SetIsCompleted false)
  (if (Utilities|IsValid _previouspiece)
    (CallFunction|Reset _previouspiece)))

(fn GetFocusTimeActive
  (return 0.0))