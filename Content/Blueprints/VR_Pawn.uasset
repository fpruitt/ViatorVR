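; VR pawn that picks what the player is looking at and sends it focus, blur and interact messages.
; Each tick a visibility trace along the camera's forward vector swaps focus with blur and focus messages, then the nearest-to-gaze registered actor overrides FocusedObject without a blur.
; That actor is chosen by the highest dot product above Threshold, from a list maintained through add and remove functions.
; The left motion controller trigger interacts with the focused object.
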(event EventBeginPlay
  (Input|EnableInput 0))

(event EventTick
  (params (DeltaSeconds :type Float%20%28single-precision%29))
  (bind _hmd_position (CallFunction|GetHMDWorldPosition))
  (bind _outhit (Collision|LineTraceByChannel _hmd_position (+ _hmd_position (* (CallFunction|GetHMDForwardVector) 1000)) "TraceTypeQuery1" false 0 "None"))
  (if (!= (Variables|Default|GetFocusedObject) (.HitActor (Collision|BreakHitResult _outhit)))
    (Class|Interactable|OnBlur(Message) (Variables|Default|GetFocusedObject))
    (Class|Interactable|OnFocus(Message) (.HitActor (Collision|BreakHitResult _outhit)))
    (Variables|Default|SetFocusedObject (.HitActor (Collision|BreakHitResult _outhit))))
  (bind _nearestobject (CallFunction|GetNearestInteractableObject))
  (Class|Interactable|OnFocus(Message) _nearestobject)
  (Variables|Default|SetFocusedObject _nearestobject))

(event Input|KeyboardEvents|MotionControllerLeftTrigger
  (params (Key :type Key%20Structure :default "AnyKey"))
  (:Pressed
    (Class|Interactable|OnInteract(Message) (Variables|Default|GetFocusedObject))))

(fn ConstructionScript)

(fn GetHMDWorldPosition
  (return (Camera|GetCameraLocation (Game|GetPlayerCameraManager 0))))

(fn GetHMDForwardVector
  (return (Transformation|GetActorForwardVector (Game|GetPlayerCameraManager 0))))

(fn GetNearestInteractableObject
  (for _array_element (Variables|Default|GetInteractableActors)
    (if (> (Math|Vector|DotProduct (CallFunction|GetHMDForwardVector) (Math|Vector|Normalize (- (Transformation|GetActorLocation _array_element) (CallFunction|GetHMDWorldPosition)))) (LocalVariables|Getthreshold))
      (LocalVariables|Setthreshold (Math|Vector|DotProduct (CallFunction|GetHMDForwardVector) (Math|Vector|Normalize (- (Transformation|GetActorLocation _array_element) (CallFunction|GetHMDWorldPosition)))))
      (LocalVariables|SetcurrentNearest _array_element)))
  (return (LocalVariables|GetcurrentNearest)))

(fn AddtoInteractableActors
  (params (Actor :type Actor%20Object%20Reference))
  (Utilities|Array|Add (Variables|Default|GetInteractableActors) Actor))

(fn RemovefromInteractableActors
  (params (Actor :type Actor%20Object%20Reference))
  (Utilities|Array|RemoveItem (Variables|Default|GetInteractableActors) Actor))