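; Pawn that teleports to the surface the camera is looking at on left mouse click.
; Each tick, a visibility line trace from the camera accepts near-flat, upward-facing hits and marks the target with a debug cylinder.
; A click moves the actor to the stored hit location, offset by the camera's relative X and Y, without sweeping.
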(event EventBeginPlay
  (Input|EnableInput (Game|GetPlayerController 0))
  (Development|PrintString "input enabled."))

(event EventActorBeginOverlap
  (params (OtherActor :type Actor%20Object%20Reference)))

(event EventTick
  (params (DeltaSeconds :type Float%20%28single-precision%29))
  (bind _camera (Variables|Default|GetCamera))
  (CallFunction|TraceGetTeleportLocation (Transformation|GetWorldLocation _camera) (Math|Vector|GetForwardVector _camera)))

(event Input|MouseEvents|LeftMouseButton
  (params (Key :type Key%20Structure :default "AnyKey"))
  (:Pressed
    (Development|PrintString "Hello")
    (if (Variables|Default|GetCanTeleport)
      (CallFunction|TeleporttoLocation (Variables|Default|GetTeleportLocation)))))

(fn ConstructionScript
  (bind _asplayer_controller (Utilities|Casting|CastToPlayerController (Pawn|GetController))))

(fn TraceGetTeleportLocation
  (params (Position :type Vector) (ForwardVector :type Vector))
  (bind _outhit (Collision|LineTraceByChannel Position (+ Position (* ForwardVector 10000)) "TraceTypeQuery1" false 0 "ForOneFrame"))
  (bind _output_get (Variables|Default|SetCanTeleport (> (Math|Vector|DotProduct (.Normal (Collision|BreakHitResult _outhit)) "0, 0,1.000000") 0.9)))
  (if _output_get
    (bind _output_get_2 (Variables|Default|SetTeleportLocation (.Location (Collision|BreakHitResult _outhit))))
    (Class|KismetSystemLibrary|DrawDebugCylinder _output_get_2 (+ _output_get_2 (* (.Normal (Collision|BreakHitResult _outhit)) 20)) 5e+01 12 "(R=1.000000,G=1.000000,B=1.000000,A=1.000000)" 0.0)))

(fn TeleporttoLocation
  (params (Location :type Vector))
  (bind _camera (Variables|Default|GetCamera))
  (bind _relativelocation (Variables|/Script/Engine.SceneComponent|GetRelativeLocation _camera))
  (Transformation|SetActorLocation (+ Location (Math|Vector|MakeVector (.x _relativelocation) (.y _relativelocation) 0.0)) false false))