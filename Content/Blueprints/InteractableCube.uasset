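; An interactable cube actor that shows its interaction state through colour.
; Focus, blur and interact events set the Color vector parameter on the Cube's materials to yellow, white and green respectively.
; GetFocusTimeActive exposes the AcceptTimer value; no timing logic runs in the cube itself.
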(event EventOnFocus
  (Rendering|Material|SetVectorParameterValueonMaterials (Variables|Default|GetCube) "Color" (Math|Conversions|ToVector(LinearColor) "(R=0.910000,G=0.865528,B=0.000000,A=1.000000)")))

(event EventOnBlur
  (Rendering|Material|SetVectorParameterValueonMaterials (Variables|Default|GetCube) "Color" "1.000000,1.000000,1.000000"))

(event EventOnInteract
  (Rendering|Material|SetVectorParameterValueonMaterials (Variables|Default|GetCube) "Color" (Math|Conversions|ToVector(LinearColor) "(R=0.083385,G=0.720000,B=0.000000,A=1.000000)")))

(fn ConstructionScript)

(fn GetFocusTimeActive
  (return (Variables|Default|GetAcceptTimer)))